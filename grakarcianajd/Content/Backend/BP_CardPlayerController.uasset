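; Card player controller that manages a deck as three card arrays: draw pile, hand and discard pile.
; DobierzKarte (draw card) moves the top draw-pile card into the hand, first refilling an empty pile by shuffling in the discard pile.
; KoniecTury (end turn) moves the whole hand to the discard pile.
; Drawing has no guard for both piles being empty, and the event graph holds only disabled stubs.
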(event EventBeginPlay)

(event EventTick
  (params (DeltaSeconds :type Float%20%28single-precision%29)))

(fn ConstructionScript)

(fn DobierzKarte
  (if (> (Utilities|Array|Length (Variables|Default|GetDrawPile)) 0)
    _
    (else
      (Variables|Default|SetDrawPile (Variables|Default|GetDiscardPile))
      (Utilities|Array|Shuffle (Variables|Default|GetDrawPile))
      (Utilities|Array|Clear (Variables|Default|GetDiscardPile))))
  (Utilities|Array|Add (Variables|Default|GetHand) (Utilities|Array|Get(acopy) (Variables|Default|GetDrawPile)))
  (Utilities|Array|RemoveIndex (Variables|Default|GetDrawPile)))

(fn KoniecTury
  (for _array_element (Variables|Default|GetHand)
    (Utilities|Array|Add (Variables|Default|GetDiscardPile) _array_element))
  (Utilities|Array|Clear (Variables|Default|GetHand)))